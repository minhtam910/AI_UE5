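; Shelter smart object whose box volume acts as an oxygen refill zone for the player character, defenders and scout enemies.
; On overlap begin it casts the entering actor to each type and starts its oxygen refill; on overlap end it resumes oxygen depletion.
; Defenders also get their peace-zone flag set on entry and cleared on exit.
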(event `self.Box.OnComponentBeginOverlap`
  (params (OverlappedComponent :type "PrimitiveComponent Object Reference") (OtherActor :type "Actor Object Reference") (OtherComp :type "PrimitiveComponent Object Reference") (OtherBodyIndex :type Integer) (bFromSweep :type Boolean) (SweepResult :type "HitResult Structure (by ref)"))
  (`|ExecutionSequence`
    (:`then_0`
      (bind _asbp_defender (cast `/Game/A_InteractObjects/AI/AI_Defender/BP_Defender` OtherActor))
      (set `/Game/A_InteractObjects/AI/AI_Defender/BP_Defender.inPeaceZone` true _asbp_defender)
      (`/Game/A_InteractObjects/AI/AI_Defender/BP_Defender.Refill Oxygen in Shelter` _asbp_defender))
    (:`then_1`
      (bind _asbp_my_tpcharacter (cast `/Game/A_InteractObjects/BP_MyTPCharacter` OtherActor))
      (`/Game/A_InteractObjects/BP_MyTPCharacter.Refill Oxygen in Shelter` _asbp_my_tpcharacter))
    (:`then_2`
      (bind _asbp_scout_enemy (cast `/Game/A_InteractObjects/AI/AI_Scout/BP_Scout_Enemy` OtherActor))
      (`/Game/A_InteractObjects/AI/AI_Scout/BP_Scout_Enemy.Refill Oxygen in Shelter` _asbp_scout_enemy))))

(event `self.Box.OnComponentEndOverlap`
  (params (OverlappedComponent :type "PrimitiveComponent Object Reference") (OtherActor :type "Actor Object Reference") (OtherComp :type "PrimitiveComponent Object Reference") (OtherBodyIndex :type Integer))
  (`|ExecutionSequence`
    (:`then_0`
      (bind _asbp_my_tpcharacter (cast `/Game/A_InteractObjects/BP_MyTPCharacter` OtherActor))
      (`/Game/A_InteractObjects/BP_MyTPCharacter.Reduce Oxygen In Game` _asbp_my_tpcharacter))
    (:`then_1`
      (bind _asbp_defender (cast `/Game/A_InteractObjects/AI/AI_Defender/BP_Defender` OtherActor))
      (set `/Game/A_InteractObjects/AI/AI_Defender/BP_Defender.inPeaceZone` false _asbp_defender)
      (`/Game/A_InteractObjects/AI/AI_Defender/BP_Defender.Reduce Oxygen In Game` _asbp_defender))
    (:`then_2`
      (bind _asbp_scout_enemy (cast `/Game/A_InteractObjects/AI/AI_Scout/BP_Scout_Enemy` OtherActor))
      (`/Game/A_InteractObjects/AI/AI_Scout/BP_Scout_Enemy.Reduce Oxygen In Game` _asbp_scout_enemy))))

(fn `UserConstructionScript`)