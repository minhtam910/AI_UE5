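; BP_Map2_Flag is a Map 2 objective actor that counts enemies reaching its box trigger.
; An overlapping scout dies and counts only if its target's display name matches this flag.
; An overlapping BP_MyTPCharacter_Enemy is destroyed and counted only at the flag named BP_Map2_TargetB.
; Both share one counter; once it hits its limit, the next arrival destroys the flag and prints "Game Over".
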(event `self.Box.OnComponentBeginOverlap`
  (params (OverlappedComponent :type "PrimitiveComponent Object Reference") (OtherActor :type "Actor Object Reference") (OtherComp :type "PrimitiveComponent Object Reference") (OtherBodyIndex :type Integer) (bFromSweep :type Boolean) (SweepResult :type "HitResult Structure (by ref)"))
  (bind _returnvalue (`KismetSystemLibrary.GetDisplayName` self))
  (`|ExecutionSequence`
    (:`then_0`
      (bind _asbp_scout_enemy (cast `/Game/A_InteractObjects/AI/AI_Scout/BP_Scout_Enemy` OtherActor))
      (bind _targetmap2 (`/Game/A_InteractObjects/AI/AI_Scout/BPI_Scout_AI.GetTargetMap2` _asbp_scout_enemy))
      (if (`KismetStringLibrary.EqualEqual_StrStr` (`KismetSystemLibrary.GetDisplayName` _targetmap2) _returnvalue)
        (`/Game/A_InteractObjects/AI/AI_Scout/BP_Scout_Enemy.Death` _asbp_scout_enemy)
        (if (< (`self.Counter`) 9) :!label _label
          (set `self.Counter` (+ (`self.Counter`) 1))
          (else
            (`self.K2_DestroyActor` self)
            (`KismetSystemLibrary.PrintString` "Game Over")))))
    (:`then_1`
      (bind _asbp_my_tpcharacter_enemy (cast `/Game/A_InteractObjects/BP_MyTPCharacter_Enemy` OtherActor))
      (if (`KismetStringLibrary.EqualEqual_StrStr` _returnvalue "BP_Map2_TargetB")
        (`self.K2_DestroyActor` _asbp_my_tpcharacter_enemy)
        (goto _label)))))

(fn `UserConstructionScript`)