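; BP_Defender is an AI defender character that chases the player, wields or sheathes a spawned hand-socketed weapon, and attacks.
; Its attack plays a montage, then sphere-traces forward to apply damage, spawn an explosion and report the hit to AI perception.
; BPCDamageSystem handles health, death ragdoll and oxygen, which looping timers drain outside and refill in shelter.
; It also exposes patrol route and movement speed functions, while several oxygen functions are stubs.
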(event `ChasePlayer`
  ;[1 1 1] Attack Flow
  ;;[1 1 1] Chase
  (`|AIMoveTo` self (0.0 0.0 0.0) (`GameplayStatics.GetPlayerCharacter` 0) 1.0 true))

(event `Attack`
  (bind _returnvalue (`self.K2_GetActorLocation`))
  ;[1 1 1] Attack Flow
  (if (not (`/Game/A_InteractObjects/DamagedSystem/BPC_DamageSystem.isDead` (`self.BPC_DamageSystem`)))
    (`|PlayMontage` (`self.Mesh`) "/Game/Characters/Mannequins/Animations/Manny/MM_Jump_Montage.MM_Jump_Montage"
      (:`OnCompleted`
        _)
      (:`OnInterrupted`
        _))
    (`self.OnAttackEnd`)
    (bind _outhit (`KismetSystemLibrary.SphereTraceSingleForObjects` :`Start` _returnvalue :`End` (+ _returnvalue (* (`self.GetActorForwardVector`) 400.0)) :`Radius` 400.0 :`ObjectTypes` (`|MakeArray` "ObjectTypeQuery3" :!type "EObjectTypeQuery Enum") :`DrawDebugType` "ForDuration" :`TraceColor` (struct :`R` 0.836153 :`G` 0.02265 :`B` 1.0 :`A` 1.0) :`TraceHitColor` (struct :`G` 0.262549 :`B` 1.0 :`A` 1.0) :`DrawTime` 1.0))
    (if true
      (bind (_bblockinghit _binitialoverlap _time _distance _location _impactpoint _normal _impactnormal _physmat _hitactor) (`GameplayStatics.BreakHitResult` _outhit))
      (bind _wasdamaged (message `/Game/A_InteractObjects/DamagedSystem/BPI_DamageAble.ReduceHealth` _hitactor (make `/Game/A_InteractObjects/DamagedSystem/S_DamageInfo` 10.0 "NewEnumerator2" "NewEnumerator1")))
      (if _wasdamaged
        (`GameplayStatics.SpawnEmitterAtLocation` "/Game/StarterContent/Particles/P_Explosion.P_Explosion" _location)
        (`AISense_Damage.ReportDamageEvent` _hitactor self 10.0 _location)))))

(event `Refill Oxygen in Shelter`
  ;[1 1 1] Oxygen Overtime
  (`KismetSystemLibrary.K2_ClearTimer` null "Reduce Oxygen when outside")
  (`KismetSystemLibrary.K2_SetTimer` null "Refill Oxygen When Inside" 1.0 true))

(event `self.ReceiveBeginPlay`
  (`KismetSystemLibrary.K2_SetTimer` null "Reduce Oxygen when outside" 1.0 true))

(event `Death`
  (bind _mesh (`self.Mesh`))
  ;[1 1 1] Damage System
  (`KismetSystemLibrary.PrintString` "Death")
  (`PrimitiveComponent.SetSimulatePhysics` _mesh true)
  (`PrimitiveComponent.SetCollisionEnabled` _mesh "QueryAndPhysics"))

(event `Reduce Oxygen In Game`
  ;[1 1 1] Oxygen Overtime
  (`KismetSystemLibrary.K2_ClearTimer` null "Refill Oxygen When Inside")
  (`KismetSystemLibrary.K2_SetTimer` null "Reduce Oxygen when outside" 1.0 true))

(event `Block`
  ;[1 1 1] Damage System
  (`KismetSystemLibrary.PrintString` "No Damage"))

(event `DamageResponse`
  (params (DamageResponse :type "/Game/A_InteractObjects/DamagedSystem/E_DamageResponse Enum" :default "NewEnumerator0"))
  ;[1 1 1] Damage System
  (`KismetSystemLibrary.PrintString` (`|GetEnumeratorNameAsString` DamageResponse)))

(event `WieldObject`
  ;[1 1 1] Weapon Flow
  ;;[1 1 1] Attach Weapon
  (bind _returnvalue (`|SpawnActorFromClass` "/Game/A_InteractObjects/BP_Weapon.BP_Weapon_C" (`self.GetTransform`) "Undefined" "OverrideRootScale" null null))
  (set `self.Weapon Actor` _returnvalue)
  (`self.K2_AttachToComponent` _returnvalue (`self.Mesh`) "hand_l_object_socket" "SnapToTarget" "SnapToTarget" "SnapToTarget" true)
  (set `self.isWieldingWeapon` true))

(event `SheathWeapon`
  ;[1 1 1] Weapon Flow
  ;;[1 1 1] Remove Weapon
  (`|PlayMontage` (`self.Mesh`) "/Game/Characters/Mannequins/Animations/Manny/MM_Jump_Montage.MM_Jump_Montage"
    (:`then`
      (`self.OnSheathWeapon`)
      (`self.K2_DestroyActor` (`self.Weapon Actor`))
      (set `self.isWieldingWeapon` false))))

(fn `getCurrentHealth`
  (returns (Health :type "Float (double-precision)"))
  (bind _health (`/Game/A_InteractObjects/DamagedSystem/BPC_DamageSystem.getCurrentHealth` (`self.BPC_DamageSystem`)))
  (return _health))

(fn `getCurrentOxygen`
  (returns (Oxygen :type "Float (double-precision)"))
  (return 0.0))

(fn `getMaxHealth`
  (returns (maxHealth :type "Float (double-precision)"))
  (bind _maxhealth (`/Game/A_InteractObjects/DamagedSystem/BPC_DamageSystem.getMaxHealth` (`self.BPC_DamageSystem`)))
  (return _maxhealth))

(fn `getMaxOxygen`
  (returns (maxOxygen :type "Float (double-precision)"))
  (return 0.0))

(fn `GetPatrolRoute`
  (returns (PatrolRoute :type "/Game/A_InteractObjects/AI/AI_Defender/BP_PatrolRoute Object Reference"))
  (return (`self.PatrolRoute`)))

(fn `Heal`
  (params (Amount :type "Float (double-precision)"))
  (returns (`New Health` :type "Float (double-precision)"))
  (bind _new_health (`/Game/A_InteractObjects/DamagedSystem/BPC_DamageSystem.Heal` (`self.BPC_DamageSystem`) Amount))
  (return _new_health))

(fn `MakeFullOxygen`
  (bind _bpc_damagesystem (`self.BPC_DamageSystem`))
  (bind _maxoxygen (`/Game/A_InteractObjects/DamagedSystem/BPC_DamageSystem.getMaxOxygen` _bpc_damagesystem))
  (set `/Game/A_InteractObjects/DamagedSystem/BPC_DamageSystem.Oxygen` _maxoxygen _bpc_damagesystem)
  (set `self.isOverheating` false))

(fn `MakeNoiseWhen`)

(fn `Reduce Oxygen when outside`
  (bind _bpc_damagesystem (`self.BPC_DamageSystem`))
  (`/Game/A_InteractObjects/DamagedSystem/BPC_DamageSystem.Reduce Oxygen` _bpc_damagesystem)
  (bind _oxygen (`/Game/A_InteractObjects/DamagedSystem/BPC_DamageSystem.getCurrentOxygen` _bpc_damagesystem))
  (if (< _oxygen 20.0)
    (bind _output_get (set `self.isOverheating` true))
    (`KismetSystemLibrary.PrintString` "Def_Low oxygen" _output_get)))

(fn `ReduceHealth`
  (params (DamagedInfo :type "/Game/A_InteractObjects/DamagedSystem/S_DamageInfo Structure"))
  (returns (WasDamaged :type Boolean))
  (bind _wasdamaged (`/Game/A_InteractObjects/DamagedSystem/BPC_DamageSystem.ReduceHealth` (`self.BPC_DamageSystem`) DamagedInfo))
  (return _wasdamaged))

(fn `ReduceOxygen`
  (return))

(fn `Refill Oxygen When Inside`
  (bind _bpc_damagesystem (`self.BPC_DamageSystem`))
  (`/Game/A_InteractObjects/DamagedSystem/BPC_DamageSystem.Rest` _bpc_damagesystem)
  (bind _oxygen (`/Game/A_InteractObjects/DamagedSystem/BPC_DamageSystem.getCurrentOxygen` _bpc_damagesystem))
  (bind _maxoxygen (`/Game/A_InteractObjects/DamagedSystem/BPC_DamageSystem.getMaxOxygen` _bpc_damagesystem))
  (if (>= _oxygen _maxoxygen)
    (set `self.isOverheating` false)))

(fn `RefillOxygen`
  (params (Amount :type "Float (double-precision)"))
  (returns (`New Oxygen` :type "Float (double-precision)"))
  (return 0.0))

(fn `SetMovementSpeed`
  (params (Speed :type "/Game/A_InteractObjects/AI/Enum/E_MovementSpeed Enum" :default "NewEnumerator0"))
  (returns (SpeedValue :type "Float (double-precision)"))
  (bind _output_get (set `CharacterMovementComponent.MaxWalkSpeed` (select `/Game/A_InteractObjects/AI/Enum/E_MovementSpeed` Speed :`NewEnumerator0` 100.0 :`NewEnumerator1` 600.0 :`NewEnumerator2` 380.0 :!type "Float (single-precision)") (`self.CharacterMovement`)))
  (return _output_get))

(fn `UserConstructionScript`
  (bind _bpc_damagesystem (`self.BPC_DamageSystem`))
  (add `/Game/A_InteractObjects/DamagedSystem/BPC_DamageSystem.OnDeath` _bpc_damagesystem (`|CreateDelegate` :!event `Death`))
  (add `/Game/A_InteractObjects/DamagedSystem/BPC_DamageSystem.OnBlock` _bpc_damagesystem (`|CreateDelegate` :!event `Block`))
  (add `/Game/A_InteractObjects/DamagedSystem/BPC_DamageSystem.OnDamageResponse` _bpc_damagesystem (`|CreateDelegate` :!event `DamageResponse`)))