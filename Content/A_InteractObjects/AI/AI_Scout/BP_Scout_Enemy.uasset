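; Scout enemy AI character that manages health and oxygen through a BPCDamageSystem component.
; Looping one-second timers drain oxygen outside or refill it in shelter, toggling an overheating flag.
; Death enables mesh physics, then asks the game mode for a map-specific respawn before destroying the actor.
; It also sets walk speeds and emits AI noise with effects; oxygen getters are stubs, and GetCurrentHealth returns max health.
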(event `self.ReceiveBeginPlay`
  (`KismetSystemLibrary.K2_SetTimer` null "Reduce Oxygen when outside" 1.0 true))

(event `Refill Oxygen in Shelter`
  ;[1 1 1] Oxygen Overtime
  (`KismetSystemLibrary.K2_ClearTimer` null "Reduce Oxygen when outside")
  (`KismetSystemLibrary.K2_SetTimer` null "Refill Oxygen When Inside" 1.0 true))

(event `Reduce Oxygen In Game`
  ;[1 1 1] Oxygen Overtime
  (`KismetSystemLibrary.K2_ClearTimer` null "Refill Oxygen When Inside")
  (`KismetSystemLibrary.K2_SetTimer` null "Reduce Oxygen when outside" 1.0 true))

(event `Death`
  (bind _mesh (`self.Mesh`))
  (`KismetSystemLibrary.PrintString` "Death")
  (`PrimitiveComponent.SetSimulatePhysics` _mesh true)
  (`PrimitiveComponent.SetCollisionEnabled` _mesh "QueryAndPhysics")
  (`KismetSystemLibrary.Delay` 1.0)
  (`KismetSystemLibrary.K2_ClearTimer` null "Reduce Oxygen when outside")
  (bind _asbp_third_person_game_mode (cast `/Game/ThirdPerson/Blueprints/BP_ThirdPersonGameMode` (`GameplayStatics.GetGameMode`)))
  (bind _returnvalue (`GameplayStatics.GetCurrentLevelName` true))
  (if (`KismetStringLibrary.EqualEqual_StrStr` _returnvalue "Map_2")
    (`/Game/ThirdPerson/Blueprints/BP_ThirdPersonGameMode.RespawnScoutTeamContext` _asbp_third_person_game_mode (`self.Map2Target`))
    (else
      (`/Game/ThirdPerson/Blueprints/BP_ThirdPersonGameMode.RespawnScout` _asbp_third_person_game_mode (`self.TargetName`))))
  (`self.K2_DestroyActor`))

(event `Block`
  (`KismetSystemLibrary.PrintString` "No Damage"))

(event `DamageResponse`
  (params (DamageResponse :type "/Game/A_InteractObjects/DamagedSystem/E_DamageResponse Enum" :default "NewEnumerator0"))
  (`KismetSystemLibrary.PrintString` (`|GetEnumeratorNameAsString` DamageResponse)))

(fn `getCurrentHealth`
  (returns (Health :type "Float (double-precision)"))
  (bind _maxhealth (`/Game/A_InteractObjects/DamagedSystem/BPC_DamageSystem.getMaxHealth` (`self.BPC_DamageSystem`)))
  (return _maxhealth))

(fn `getCurrentOxygen`
  (returns (Oxygen :type "Float (double-precision)"))
  (return 0.0))

(fn `getMaxHealth`
  (returns (maxHealth :type "Float (double-precision)"))
  (bind _maxhealth (`/Game/A_InteractObjects/DamagedSystem/BPC_DamageSystem.getMaxHealth` (`self.BPC_DamageSystem`)))
  (return _maxhealth))

(fn `getMaxOxygen`
  (returns (maxOxygen :type "Float (double-precision)"))
  (return 0.0))

(fn `GetTarget`
  (returns (Target :type "/Game/A_InteractObjects/BP_Target Object Reference"))
  (return (`self.TargetName`)))

(fn `GetTargetMap2`
  (returns (TargetMap2 :type "/Game/A_InteractObjects/Map2/BP_Map2_Flag Object Reference"))
  (return (`self.Map2Target`)))

(fn `Heal`
  (params (Amount :type "Float (double-precision)"))
  (returns (`New Health` :type "Float (double-precision)"))
  (bind _new_health (`/Game/A_InteractObjects/DamagedSystem/BPC_DamageSystem.Heal` (`self.BPC_DamageSystem`) Amount))
  (return _new_health))

(fn `Reduce Oxygen when outside`
  (bind _bpc_damagesystem (`self.BPC_DamageSystem`))
  (`/Game/A_InteractObjects/DamagedSystem/BPC_DamageSystem.Reduce Oxygen` _bpc_damagesystem)
  (bind _oxygen (`/Game/A_InteractObjects/DamagedSystem/BPC_DamageSystem.getCurrentOxygen` _bpc_damagesystem))
  (if (< _oxygen 20.0)
    (bind _output_get (set `self.isOverheating` true))
    (`KismetSystemLibrary.PrintString` "Scout_Low oxygen" _output_get)))

(fn `ReduceHealth`
  (params (DamagedInfo :type "/Game/A_InteractObjects/DamagedSystem/S_DamageInfo Structure"))
  (returns (WasDamaged :type Boolean))
  (bind _wasdamaged (`/Game/A_InteractObjects/DamagedSystem/BPC_DamageSystem.ReduceHealth` (`self.BPC_DamageSystem`) DamagedInfo))
  (return _wasdamaged))

(fn `Refill Oxygen When Inside`
  (bind _bpc_damagesystem (`self.BPC_DamageSystem`))
  (`/Game/A_InteractObjects/DamagedSystem/BPC_DamageSystem.Rest` _bpc_damagesystem)
  (bind _oxygen (`/Game/A_InteractObjects/DamagedSystem/BPC_DamageSystem.getCurrentOxygen` _bpc_damagesystem))
  (bind _maxoxygen (`/Game/A_InteractObjects/DamagedSystem/BPC_DamageSystem.getMaxOxygen` _bpc_damagesystem))
  (if (>= _oxygen _maxoxygen)
    (set `self.isOverheating` false)))

(fn `RefillOxygen`
  (params (Amount :type "Float (double-precision)"))
  (returns (`New Oxygen` :type "Float (double-precision)"))
  (return 0.0))

(fn `SetMovementSpeed`
  (params (Speed :type "/Game/A_InteractObjects/AI/Enum/E_MovementSpeed Enum" :default "NewEnumerator0"))
  (returns (SpeedValue :type "Float (double-precision)"))
  (bind _output_get (set `CharacterMovementComponent.MaxWalkSpeed` (select `/Game/A_InteractObjects/AI/Enum/E_MovementSpeed` Speed :`NewEnumerator0` 150.0 :`NewEnumerator1` 450.0 :`NewEnumerator2` 350.0 :!type "Float (single-precision)") (`self.CharacterMovement`)))
  (return _output_get))

(fn `Step On Noisy Thing`
  (bind _returnvalue (`self.K2_GetActorLocation` self))
  (`self.MakeNoise` self 1.0 null _returnvalue 0.0 "None")
  (`GameplayStatics.SpawnEmitterAtLocation` null _returnvalue)
  (`GameplayStatics.PlaySoundAtLocation` "/Game/A_InteractObjects/SmartObject/falling-branch.falling-branch" _returnvalue (struct) 1.0 1.0 0.0 null null null null))

(fn `UserConstructionScript`
  (bind _bpc_damagesystem (`self.BPC_DamageSystem`))
  (add `/Game/A_InteractObjects/DamagedSystem/BPC_DamageSystem.OnDeath` _bpc_damagesystem (`|CreateDelegate` :!event `Death`))
  (add `/Game/A_InteractObjects/DamagedSystem/BPC_DamageSystem.OnBlock` _bpc_damagesystem (`|CreateDelegate` :!event `Block`))
  (add `/Game/A_InteractObjects/DamagedSystem/BPC_DamageSystem.OnDeath` _bpc_damagesystem (`|CreateDelegate` :!event `Death`)))