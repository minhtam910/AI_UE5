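; Scout enemy character that can chase player 0 through AI MoveTo and switch among walk, jog and sprint speeds.
; Health, healing and damage calls forward to BPCDamageSystem, though GetCurrentHealth returns max health and oxygen functions are zero-returning stubs.
; The construction script binds the component's death and block delegates, with OnDeath bound twice.
; Death ragdolls the mesh with collision enabled, while block and damage response events only print debug text.
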(event `ChasePlayer`
  (`|AIMoveTo` self (0.0 0.0 0.0) (`GameplayStatics.GetPlayerCharacter` 0)))

(event `Death`
  (bind _mesh (`self.Mesh`))
  (`KismetSystemLibrary.PrintString` "Death")
  (`PrimitiveComponent.SetSimulatePhysics` _mesh true)
  (`PrimitiveComponent.SetCollisionEnabled` _mesh "QueryAndPhysics"))

(event `Block`
  (`KismetSystemLibrary.PrintString` "No Damage"))

(event `DamageResponse`
  (params (DamageResponse :type "/Game/A_InteractObjects/DamagedSystem/E_DamageResponse Enum" :default "NewEnumerator0"))
  (`KismetSystemLibrary.PrintString` (`|GetEnumeratorNameAsString` DamageResponse)))

(fn `getCurrentHealth`
  (returns (Health :type "Float (double-precision)"))
  (bind _maxhealth (`/Game/A_InteractObjects/DamagedSystem/BPC_DamageSystem.getMaxHealth` (`self.BPC_DamageSystem`)))
  (return _maxhealth))

(fn `getCurrentOxygen`
  (returns (Oxygen :type "Float (double-precision)"))
  (return 0.0))

(fn `getMaxHealth`
  (returns (maxHealth :type "Float (double-precision)"))
  (bind _maxhealth (`/Game/A_InteractObjects/DamagedSystem/BPC_DamageSystem.getMaxHealth` (`self.BPC_DamageSystem`)))
  (return _maxhealth))

(fn `getMaxOxygen`
  (returns (maxOxygen :type "Float (double-precision)"))
  (return 0.0))

(fn `Heal`
  (params (Amount :type "Float (double-precision)"))
  (returns (`New Health` :type "Float (double-precision)"))
  (bind _new_health (`/Game/A_InteractObjects/DamagedSystem/BPC_DamageSystem.Heal` (`self.BPC_DamageSystem`) Amount))
  (return _new_health))

(fn `ReduceHealth`
  (params (DamagedInfo :type "/Game/A_InteractObjects/DamagedSystem/S_DamageInfo Structure"))
  (returns (WasDamaged :type Boolean))
  (bind _wasdamaged (`/Game/A_InteractObjects/DamagedSystem/BPC_DamageSystem.ReduceHealth` (`self.BPC_DamageSystem`) DamagedInfo))
  (return _wasdamaged))

(fn `RefillOxygen`
  (params (Amount :type "Float (double-precision)"))
  (returns (`New Oxygen` :type "Float (double-precision)"))
  (return 0.0))

(fn `SetMovementSpeed`
  (params (Speed :type "/Game/A_InteractObjects/AI/Enum/E_MovementSpeed Enum" :default "NewEnumerator0"))
  (returns (SpeedValue :type "Float (double-precision)"))
  (bind _output_get (set `CharacterMovementComponent.MaxWalkSpeed` (select `/Game/A_InteractObjects/AI/Enum/E_MovementSpeed` Speed :`NewEnumerator0` 150.0 :`NewEnumerator1` 500.0 :`NewEnumerator2` 350.0 :!type "Float (single-precision)") (`self.CharacterMovement`)))
  (return _output_get))

(fn `UserConstructionScript`
  (bind _bpc_damagesystem (`self.BPC_DamageSystem`))
  (add `/Game/A_InteractObjects/DamagedSystem/BPC_DamageSystem.OnDeath` _bpc_damagesystem (`|CreateDelegate` :!event `Death`))
  (add `/Game/A_InteractObjects/DamagedSystem/BPC_DamageSystem.OnBlock` _bpc_damagesystem (`|CreateDelegate` :!event `Block`))
  (add `/Game/A_InteractObjects/DamagedSystem/BPC_DamageSystem.OnDeath` _bpc_damagesystem (`|CreateDelegate` :!event `Death`)))