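; BP_Target is a target actor whose box overlap reacts to enemy characters reaching it.
; Each BP_Scout_Enemy that enters is destroyed and counted; the third destroys the target and calls Map1CheckEnd on BP_ThirdPersonGameMode.
; A BP_MyTPCharacter_Enemy entering instead clears all scouts and defenders, pauses the game and shows the fading WBP_Level1 widget with the mouse cursor.
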(event `self.Box.OnComponentBeginOverlap`
  (params (OverlappedComponent :type "PrimitiveComponent Object Reference") (OtherActor :type "Actor Object Reference") (OtherComp :type "PrimitiveComponent Object Reference") (OtherBodyIndex :type Integer) (bFromSweep :type Boolean) (SweepResult :type "HitResult Structure (by ref)"))
  (bind _returnvalue (`GameplayStatics.GetPlayerController` 0))
  (bind _counter (`self.Counter`))
  (`|ExecutionSequence`
    (:`then_0`
      (bind _asbp_scout_enemy (cast `/Game/A_InteractObjects/AI/AI_Scout/BP_Scout_Enemy` OtherActor))
      (`self.K2_DestroyActor` _asbp_scout_enemy)
      (if (< _counter 2)
        (set `self.Counter` (+ _counter 1))
        (else
          (`self.K2_DestroyActor`)
          (bind _asbp_third_person_game_mode (cast `/Game/ThirdPerson/Blueprints/BP_ThirdPersonGameMode` (`GameplayStatics.GetGameMode`)))
          (`/Game/ThirdPerson/Blueprints/BP_ThirdPersonGameMode.Map1_CheckEnd` _asbp_third_person_game_mode))))
    (:`then_1`
      (bind _asbp_my_tpcharacter_enemy (cast `/Game/A_InteractObjects/BP_MyTPCharacter_Enemy` OtherActor))
      (bind _outactors (`GameplayStatics.GetAllActorsOfClass` "/Game/A_InteractObjects/AI/AI_Scout/BP_Scout_Enemy.BP_Scout_Enemy_C"))
      (for _index (range (+ (`KismetArrayLibrary.Array_Length` _outactors) 1))
        (`self.K2_DestroyActor` (`|GetArrayItem` _outactors _index)))
      (bind _outactors_2 (`GameplayStatics.GetAllActorsOfClass` "/Game/A_InteractObjects/AI/AI_Defender/BP_Defender.BP_Defender_C"))
      (for _index_2 (range (+ (`KismetArrayLibrary.Array_Length` _outactors_2) 1))
        (`self.K2_DestroyActor` (`|GetArrayItem` _outactors_2 _index_2)))
      (set `PlayerController.bShowMouseCursor` true _returnvalue)
      (`GameplayStatics.SetGamePaused` true)
      (bind _returnvalue_2 (`|CreateWidget` "/Game/UI/LevelWidgets/WBP_Level1.WBP_Level1_C" _returnvalue))
      (`UserWidget.AddToViewport` _returnvalue_2 0)
      (`/Game/UI/LevelWidgets/WBP_Level1.FadeAnim` _returnvalue_2))))

(fn `UserConstructionScript`)