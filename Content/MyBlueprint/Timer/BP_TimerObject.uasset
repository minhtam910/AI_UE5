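; BP_TimerObject is the round countdown timer that decides a win or loss when time runs out.
; Tick passes through a one-second Delay to count Minutes and Seconds down.
; At zero it pauses the game and reads AttachToPlayer on the first BP_Crown found.
; If attached, it plays a sound, shows WBP_Won and calls QuitGame after a further Delay; otherwise it shows WBP_Lose.
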(event `self.ReceiveTick`
  (params (DeltaSeconds :type "Float (single-precision)"))
  ;[1 1 1] Timer
  (`KismetSystemLibrary.Delay` 1.0)
  (if (== (`self.Seconds`) 0)
    (if (== (`self.Minutes`) 0)
      (bind _outactors (`GameplayStatics.GetAllActorsOfClass` "/Game/A_InteractObjects/Map3/BP_Crown.BP_Crown_C"))
      (if (`/Game/A_InteractObjects/Map3/BP_Crown.AttachToPlayer` (`|GetArrayItem` _outactors))
        (`GameplayStatics.SetGamePaused` true)
        (`KismetSystemLibrary.PrintString` "Attach to player")
        (`GameplayStatics.PlaySound2D` "/Game/Audio/WinningSong/tape-saturated-drum-loop-96bpm-142842.tape-saturated-drum-loop-96bpm-142842" 1.0 1.0 0.0 null null)
        (bind _returnvalue (`|CreateWidget` "/Game/UI/GameWidgets/WBP_Won.WBP_Won_C"))
        (`UserWidget.AddToViewport` _returnvalue 0)
        (`KismetSystemLibrary.Delay` 10.0)
        (`KismetSystemLibrary.QuitGame` null "Quit")
        (else
          (`GameplayStatics.SetGamePaused` true)
          (`KismetSystemLibrary.PrintString` "No attach")
          (bind _returnvalue_2 (`|CreateWidget` "/Game/WBP_Lose.WBP_Lose_C"))
          (`UserWidget.AddToViewport` _returnvalue_2 0)))
      (else
        (set `self.Seconds` 59)
        (set `self.Minutes` (- (`self.Minutes`) 1))))
    (else
      (set `self.Seconds` (- (`self.Seconds`) 1)))))

(fn `UserConstructionScript`)